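; Unicorn weapon component that implements a hold-to-charge shot for the first-person character, with range growing while charging.
; Input start plays an attached charging sound, while trigger calls extend AttackRange along X, throttled by a short Delay.
; Exceeding the maximum pauses the sound.
; Release pauses it too, multicasts the effect at the calculated spawn position scaled by AttackRange, resets the range and multicasts the shot sound.
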(event Custom|EncreaseAttacRange
  (Utilities|FlowControl|Delay 0.2)
  (if (> (.x (Variables|Default|GetAttackRange)) (Variables|Default|GetMaxAttacRange))
    (Development|PrintString "Voluting time")
    (CallFunction|ClientChargedWeapon)
    (else
      (bind _output_get (Variables|Default|SetAttackRange (+ (Variables|Default|GetAttackRange) (Math|Vector|MakeVector 5.0 0.0 0.0))))
      (Development|PrintText (Utilities|Text|ToText(String) _output_get)))))

(event Custom|ClientOnChargeWeapon
  (bind _returnvalue (Audio|SpawnSoundAttached "/Game/Sounds/Draining-Water-Down-Sink-CloseDistance-1-www_FesliyanStudios_com.Draining-Water-Down-Sink-CloseDistance-1-www_FesliyanStudios_com" self "None" "0, 0, 0" "0, 0, 0" "KeepRelativeOffset" false 1.0 1.0 0.0 0 0))
  (bind _output_get (Variables|Components|SetChargingSound _returnvalue))
  (Audio|Components|Audio|Play _output_get 0.0))

(event Custom|ClientChargedWeapon
  (Class|AudioComponent|SetPaused (Variables|Components|GetChargingSound) true))

(event EventOnInputStart
  (CallFunction|ClientonChargeWeapon))

(event EventOnTriggerShoot
  (params (rotator :type Rotator :default "0, 0, 0"))
  (CallFunction|EncreaseAttacRange))

(event EventOnInputComplete
  (CallFunction|ClientChargedWeapon)
  (CallFunction|Shooting)
  (Variables|Default|SetAttackRange "10.000000,5.000000,5.000000")
  (Default|MulticastonShoot (Variables|Default|GetFirst%20PersonCharacter) (Variables|Default|GetSound)))

(event EventShooting
  (params (Transform :type Transform))
  (Default|MulticastAfterShoot (Variables|Default|GetFirst%20PersonCharacter) (Variables|Default|GetEffect) (.location (CallFunction|CalculateSpawnPosion (stale EventOnTriggerShoot rotator))) (Variables|Default|GetAttackRange)))

(fn AttachWeaponComponent
  (params (NewMesh :type Skeletal%20Mesh%20Object%20Reference))
  (|CallParentFunction NewMesh))