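; GameState Blueprint that shows a kill popup naming the killed player.
; BeginPlay creates the Killpopup widget, adds it to the viewport and prints a debug "Hello".
; OnKill resolves the killed actor's PlayerState name through its pawn's BP_FirstPersonPlayerController, then WidgetSetUp passes it to the popup.
; The lookup stops if either the pawn or controller cast fails.
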(event Custom|OnKill
  (params (Killed :type BP%20First%20Person%20Character%20Object%20Reference))
  (bind _name (Default|GetKilledName Killed))
  (CallFunction|WidgetSetUp _name))

(event Custom|WidgetSetUp
  (params (Name :type Text))
  (Default|SetupKillpopup (Variables|Default|GetKillpopup) Name))

(event EventBeginPlay
  (bind _returnvalue (UserInterface|CreateWidget "/Game/UI/Killpopup.Killpopup_C"))
  (bind _output_get (Variables|Default|SetKillpopup _returnvalue))
  (UserInterface|Viewport|AddtoViewport _output_get 0)
  (Development|PrintText "Hello"))

(fn ConstructionScript)

(fn GetKilledName
  (params (Actor :type Actor%20Object%20Reference))
  (bind _aspawn (Utilities|Casting|CastToPawn Actor))
  (bind _asbp_first_person_player_controller (Utilities|Casting|CastToBP_FirstPersonPlayerController (Pawn|GetController _aspawn)))
  (return (Utilities|Text|ToText(String) (PlayerState|GetPlayerName (Variables|/Script/Engine.Controller|GetPlayerState _asbp_first_person_player_controller)))))