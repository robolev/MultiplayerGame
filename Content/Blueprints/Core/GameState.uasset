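; GameState Blueprint that announces kills by sending the killed player's name to player characters.
; OnKill resolves the name from the killed Pawn's BP_FirstPersonPlayerController and its PlayerState via GetKilledName.
; WidgetSetUp then loops over every BP_FirstPersonCharacter from GetAllActorsOfClass and calls ClientAddKillfeed on each.
; A disconnected branch that creates a Killpopup widget in the viewport never runs.
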(event Custom|OnKill
  (params (Killed :type BP%20First%20Person%20Character%20Object%20Reference))
  (bind _name (CallFunction|GetKilledName Killed))
  (CallFunction|WidgetSetUp _name))

(event Custom|WidgetSetUp
  (params (Name :type Text))
  (bind _outactors (Actor|GetAllActorsOfClass "/Game/FirstPerson/Blueprints/BP_FirstPersonCharacter.BP_FirstPersonCharacter_C"))
  (for _array_element _outactors
    (Default|ClientAddKillfeed _array_element Name)))

(event EventBeginPlay)

(fn ConstructionScript)

(fn GetKilledName
  (params (Actor :type Actor%20Object%20Reference))
  (bind _aspawn (Utilities|Casting|CastToPawn Actor))
  (bind _asbp_first_person_player_controller (Utilities|Casting|CastToBP_FirstPersonPlayerController (Pawn|GetController _aspawn)))
  (return (Utilities|Text|ToText(String) (PlayerState|GetPlayerName (Variables|/Script/Engine.Controller|GetPlayerState _asbp_first_person_player_controller)))))